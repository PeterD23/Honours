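; BP_Planet is a procedurally configured planet actor that orbits a given star and spins on its axis.
; InitPlanet sets size, orbit radius, a distance-inverse angular speed and a seeded start angle.
; It then colours a dynamic material instance by type: fixed palettes for Rock and Earth, seeded pale tints for ice.
; Tick advances the angle, placing the planet on a flat circle around the star while adding yaw.
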(event EventTick
  (params (DeltaSeconds :type Float%20%28single-precision%29))
  (Variables|Default|SetAngle (+ (Variables|Default|GetAngle) (* (Variables|Default|GetVelocity) DeltaSeconds)))
  (Transformation|SetActorTransform (Math|Transform|MakeTransform (+ (Transformation|GetActorLocation (Variables|Default|GetSTAR)) (Math|Vector|MakeVector (* (Variables|Default|GetOrbitRadius) (Math|Trig|Sin(Degrees) (Variables|Default|GetAngle))) (* (Variables|Default|GetOrbitRadius) (Math|Trig|Cos(Degrees) (Variables|Default|GetAngle))) 0.0)) (Math|Rotator|MakeRotator 0.0 0.0 (+ (.Yaw (Math|Rotator|BreakRotator (Transformation|GetActorRotation))) (* (/ DeltaSeconds (Variables|Default|GetRevolutionSeconds)) 3.6e+02))))))

(event EventBeginPlay)

(event Collision|EventActorBeginOverlap
  (params (OtherActor :type Actor%20Object%20Reference)))

(fn ConstructionScript
  (bind _returnvalue (Rendering|Material|CreateDynamicMaterialInstance (Variables|Default|GetPlanet) 0 0 :!class /Script/Engine.PrimitiveComponent))
  (Variables|Default|SetMaterial _returnvalue))

(fn InitPlanet
  (params (Planet%20Type :type String) (Size :type Integer) (Seed :type Random%20Stream%20Structure) (Distance :type Float%20%28single-precision%29) (STAR :type BP%20Star%20Object%20Reference))
  (bind _returnvalue (Math|Random|RandomIntegerinRangefromStream 0 360 Seed))
  ;[1 1 1] Set Scale
  (bind _output_get (Variables|Default|SetSize Size))
  (Variables|Default|SetSTAR STAR)
  (Transformation|SetWorldScale3D (Variables|Default|GetPlanet) (Math|Vector|MakeVector (Math|Conversions|ToFloat(Integer) _output_get) (Math|Conversions|ToFloat(Integer) _output_get) (Math|Conversions|ToFloat(Integer) _output_get)))
  (bind _output_get_2 (Variables|Default|SetOrbitRadius Distance))
  (Variables|Default|SetVelocity (/ 1e+04 _output_get_2))
  (Variables|Default|SetAngle (Math|Conversions|ToFloat(Integer) _returnvalue))
  ;[1 1 1] Set Colour and Location
  (Development|PrintString (Utilities|String|ToString(Integer) _returnvalue) true true "(R=0.000000,G=0.660000,B=1.000000,A=1.000000)" 1e+01)
  (Rendering|Material|SetMaterial (Variables|Default|GetPlanet) 0 (Variables|Default|GetMaterial))
  (if (Utilities|Enum|Equal(Enum) Planet%20Type "Rock")
    (bind _seed_out (CallFunction|RockType Seed))
    (return _seed_out)
    (elif (Utilities|Enum|Equal(Enum) Planet%20Type "Earth")
      (bind _seed_out_2 (CallFunction|HabitableType Seed))
      (return _seed_out_2)
      (else
        (bind _seed_out_3 (CallFunction|IceType Seed))
        (return _seed_out_3)))))

(fn IceType
  (params (Seed :type Random%20Stream%20Structure))
  (bind _returnvalue (Math|Random|RandomFloatinRangefromStream 0.4 1.0 Seed))
  (bind _returnvalue_2 (Math|Random|RandomFloatinRangefromStream 0.6 1.0 Seed))
  (bind _returnvalue_3 (Math|Random|RandomFloatinRangefromStream 0.9 1.0 Seed))
  (bind _returnvalue_4 (Math|Random|RandomFloatinRangefromStream 0.8 1.0 Seed))
  (bind _material (Variables|Default|GetMaterial))
  (Rendering|Material|SetVectorParameterValue _material "Color 1" (Math|Color|MakeColor _returnvalue_3 _returnvalue_3 _returnvalue_3) :!class /Script/Engine.MaterialInstanceDynamic)
  (Rendering|Material|SetVectorParameterValue _material "Color 2" (Math|Color|MakeColor _returnvalue_4 _returnvalue_4 _returnvalue_4) :!class /Script/Engine.MaterialInstanceDynamic)
  (Rendering|Material|SetVectorParameterValue _material "Color 3" (Math|Color|MakeColor _returnvalue_2 _returnvalue_2 _returnvalue_2) :!class /Script/Engine.MaterialInstanceDynamic)
  (Rendering|Material|SetVectorParameterValue _material "Color 4" (Math|Color|MakeColor _returnvalue _returnvalue _returnvalue) :!class /Script/Engine.MaterialInstanceDynamic)
  (return Seed))

(fn HabitableType
  (params (Seed :type Random%20Stream%20Structure))
  (bind _material (Variables|Default|GetMaterial))
  (Rendering|Material|SetVectorParameterValue _material "Color 1" "(R=0.000000,G=0.884117,B=1.000000,A=1.000000)" :!class /Script/Engine.MaterialInstanceDynamic)
  (Rendering|Material|SetVectorParameterValue _material "Color 2" "(R=0.210600,G=0.780000,B=0.302747,A=1.000000)" :!class /Script/Engine.MaterialInstanceDynamic)
  (Rendering|Material|SetVectorParameterValue _material "Color 3" "(R=0.169598,G=0.540000,B=0.265845,A=1.000000)" :!class /Script/Engine.MaterialInstanceDynamic)
  (Rendering|Material|SetVectorParameterValue _material "Color 4" "(R=0.852973,G=0.870000,B=0.100050,A=1.000000)" :!class /Script/Engine.MaterialInstanceDynamic)
  (return Seed))

(fn RockType
  (params (Seed :type Random%20Stream%20Structure))
  (bind _material (Variables|Default|GetMaterial))
  (Rendering|Material|SetVectorParameterValue _material "Color 1" "(R=0.000000,G=0.000000,B=0.000000,A=1.000000)" :!class /Script/Engine.MaterialInstanceDynamic)
  (Rendering|Material|SetVectorParameterValue _material "Color 2" "(R=0.000000,G=0.000000,B=0.000000,A=1.000000)" :!class /Script/Engine.MaterialInstanceDynamic)
  (Rendering|Material|SetVectorParameterValue _material "Color 3" "(R=1.000000,G=0.000000,B=0.000000,A=1.000000)" :!class /Script/Engine.MaterialInstanceDynamic)
  (Rendering|Material|SetVectorParameterValue _material "Color 4" "(R=1.000000,G=0.000000,B=0.000000,A=1.000000)" :!class /Script/Engine.MaterialInstanceDynamic)
  (return Seed))