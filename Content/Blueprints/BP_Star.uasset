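; Procedurally generated star actor that rolls physical properties for a given spectral type, O through M.
; InitStar uses a seeded random stream to pick temperature, mass, radius and luminosity within per-type ranges, then derives the classification label and colours a dynamic material.
; It computes a habitable zone from luminosity and temperature, scales the mesh by radius, centres the actor at the origin, offsets the camera and sets light intensity and temperature.
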(event EventBeginPlay)

(event EventActorBeginOverlap
  (params (OtherActor :type Actor%20Object%20Reference)))

(event EventTick
  (params (DeltaSeconds :type Float%20%28single-precision%29)))

(fn ConstructionScript
  (bind _returnvalue (Rendering|Material|CreateDynamicMaterialInstance (Variables|Default|GetStar) 0 "/Game/Materials/M_StarGen.M_StarGen" :!class /Script/Engine.PrimitiveComponent))
  (Variables|Default|SetMaterial _returnvalue))

(fn InitStar
  (params (Star%20Type :type Integer) (Seed :type Random%20Stream%20Structure))
  (bind _radius (Variables|Default|GetRadius))
  (bind _lighting (Variables|Default|GetLighting))
  (bind _returnvalue (* _radius 6.957))
  ;[1 1 1] Set Type and Info (Spectral Classification, Temperature, Radius, Mass, Luminosity)
  (bind _seedout (CallFunction|SettingStarInfoandColour Star%20Type Seed))
  (CallFunction|SetHabitableZone)
  ;[1 1 1] Set Scale and Location
  (Transformation|SetWorldScale3D (Variables|Default|GetStar) (Math|Vector|MakeVector _returnvalue _returnvalue _returnvalue))
  (Transformation|SetActorLocation "0.000000,0.000000, 0" false false)
  (Transformation|SetRelativeLocation (Variables|Default|GetCamera) (+ (Variables|/Script/Engine.SceneComponent|GetRelativeLocation (Variables|Default|GetStar)) (Math|Vector|MakeVector 0.0 (* _returnvalue 1e+02) 0.0)) false false)
  (Rendering|Components|Light|SetIntensity _lighting (Math|Float|Clamp(Float) (* (Variables|Default|GetLuminosity) 1e+06) 0.0 1e+08))
  (Class|LightComponent|SetTemperature _lighting (Math|Conversions|ToFloat(Integer) (Variables|Default|GetTemperature)))
  (return _seedout))

(fn SetColour
  (params (R :type Float%20%28single-precision%29) (G :type Float%20%28single-precision%29) (B :type Float%20%28single-precision%29))
  (Rendering|Material|SetVectorParameterValue (Variables|Default|GetMaterial) "Color" (Math|Color|MakeColor R G B) :!class /Script/Engine.MaterialInstanceDynamic)
  (return))

(fn SettingStarInfoandColour
  (params (Type :type Integer) (Seed :type Random%20Stream%20Structure))
  (bind _output_get (Variables|Default|SetType Type))
  ;[1 1 1] Horrendous Branches
  (if (== _output_get 0)
    (bind _seedout (CallFunction|OType Seed))
    (return _seedout)
    (elif (== _output_get 1)
      (bind _seed_out (CallFunction|BType Seed))
      (return _seed_out)
      (elif (== _output_get 2)
        (bind _seed_out_2 (CallFunction|AType Seed))
        (return _seed_out_2)
        (elif (== _output_get 3)
          (bind _seed_out_3 (CallFunction|FType Seed))
          (return _seed_out_3)
          (elif (== _output_get 4)
            (bind _seed_out_4 (CallFunction|GType Seed))
            (return _seed_out_4)
            (elif (== _output_get 5)
              (bind _seed_out_5 (CallFunction|KType Seed))
              (return _seed_out_5)
              (else
                (bind _seed_out_6 (CallFunction|MType Seed))
                (return _seed_out_6)))))))))

(fn SetTemp
  (params (Min :type Integer) (Max :type Integer) (Seed :type Random%20Stream%20Structure))
  (Variables|Default|SetTemperature (Math|Random|RandomIntegerinRangefromStream Min Max Seed)))

(fn SetRadius
  (params (Min :type Float%20%28single-precision%29) (Max :type Float%20%28single-precision%29) (Seed :type Random%20Stream%20Structure))
  (Variables|Default|SetRadius (Math|Random|RandomFloatinRangefromStream Min Max Seed)))

(fn SetMass
  (params (Min :type Float%20%28single-precision%29) (Max :type Float%20%28single-precision%29) (Seed :type Random%20Stream%20Structure))
  (Variables|Default|SetMass (Math|Random|RandomFloatinRangefromStream Min Max Seed)))

(fn SetLuminosity
  (params (Min :type Float%20%28single-precision%29) (Max :type Float%20%28single-precision%29) (Seed :type Random%20Stream%20Structure))
  (Variables|Default|SetLuminosity (Math|Random|RandomFloatinRangefromStream Min Max Seed)))

(fn OType
  (params (Seed :type Random%20Stream%20Structure))
  (CallFunction|SetTemp 30000 60000 Seed)
  (CallFunction|SetMass 16.0 32.0 Seed)
  (CallFunction|SetRadius 6.6 13.2 Seed)
  (CallFunction|SetLuminosity 3e+04 6e+04 Seed)
  (CallFunction|SetColour 0.61 0.69 1.0)
  ;[1 1 1] Set Spectral Classifcation (e.g. O5)
  (Variables|Default|SetSpectral%20Classification (Utilities|String|Append "O" (Utilities|String|ToString(Integer) (|(Abs((1-x))) (- (/ (Variables|Default|GetTemperature) 6000) 1)))))
  (return Seed))

(fn BType
  (params (Seed :type Random%20Stream%20Structure))
  (CallFunction|SetTemp 15000 30000 Seed)
  (CallFunction|SetMass 2.1 16.0 Seed)
  (CallFunction|SetRadius 1.8 6.6 Seed)
  (CallFunction|SetLuminosity 25.0 3e+04 Seed)
  (CallFunction|SetColour 0.67 0.75 1.0)
  ;[1 1 1] Set Spectral Classifcation (e.g. O5)
  (Variables|Default|SetSpectral%20Classification (Utilities|String|Append "B" (Utilities|String|ToString(Integer) (|(Abs((1-x))) (- (/ (Variables|Default|GetTemperature) 3000) 1)))))
  (return Seed))

(fn AType
  (params (Seed :type Random%20Stream%20Structure))
  (CallFunction|SetTemp 7500 15000 Seed)
  (CallFunction|SetMass 1.4 2.1 Seed)
  (CallFunction|SetRadius 1.4 1.8 Seed)
  (CallFunction|SetLuminosity 5.0 25.0 Seed)
  (CallFunction|SetColour 0.75 0.85 1.0)
  ;[1 1 1] Set Spectral Classifcation (e.g. O5)
  (Variables|Default|SetSpectral%20Classification (Utilities|String|Append "A" (Utilities|String|ToString(Integer) (|(Abs((1-x))) (- (/ (Variables|Default|GetTemperature) 1500) 1)))))
  (return ""))

(fn FType
  (params (Seed :type Random%20Stream%20Structure))
  (CallFunction|SetTemp 6000 7500 Seed)
  (CallFunction|SetMass 1.04 1.4 Seed)
  (CallFunction|SetRadius 1.15 1.4 Seed)
  (CallFunction|SetLuminosity 1.5 5.0 Seed)
  (CallFunction|SetColour 0.98 0.97 1.0)
  ;[1 1 1] Set Spectral Classifcation (e.g. O5)
  (Variables|Default|SetSpectral%20Classification (Utilities|String|Append "F" (Utilities|String|ToString(Integer) (|(Abs((1-x))) (- (/ (Variables|Default|GetTemperature) 750) 1)))))
  (return Seed))

(fn GType
  (params (Seed :type Random%20Stream%20Structure))
  (CallFunction|SetTemp 5200 6000 Seed)
  (CallFunction|SetMass 0.8 1.04 Seed)
  (CallFunction|SetRadius 0.96 1.15 Seed)
  (CallFunction|SetLuminosity 0.6 1.5 Seed)
  (CallFunction|SetColour 1.0 0.96 0.91)
  ;[1 1 1] Set Spectral Classifcation (e.g. O5)
  (Variables|Default|SetSpectral%20Classification (Utilities|String|Append "G" (Utilities|String|ToString(Integer) (|(Abs((1-x))) (- (/ (Variables|Default|GetTemperature) 600) 1)))))
  (return ""))

(fn KType
  (params (Seed :type Random%20Stream%20Structure))
  (CallFunction|SetTemp 3700 5200 Seed)
  (CallFunction|SetMass 0.45 0.8 Seed)
  (CallFunction|SetRadius 0.7 0.96 Seed)
  (CallFunction|SetLuminosity 0.08 0.6 Seed)
  (CallFunction|SetColour 1.0 0.87 0.71)
  ;[1 1 1] Set Spectral Classifcation (e.g. O5)
  (Variables|Default|SetSpectral%20Classification (Utilities|String|Append "K" (Utilities|String|ToString(Integer) (|(Abs((1-x))) (- (/ (Variables|Default|GetTemperature) 520) 1)))))
  (return Seed))

(fn MType
  (params (Seed :type Random%20Stream%20Structure))
  (CallFunction|SetTemp 2400 3700 Seed)
  (CallFunction|SetMass 0.08 0.45 Seed)
  (CallFunction|SetRadius 0.35 0.7 Seed)
  (CallFunction|SetLuminosity 0.04 0.08 Seed)
  (CallFunction|SetColour 1.0 0.27 0.0)
  (Class|LightComponent|SetTemperature (Variables|Default|GetLighting) (Math|Conversions|ToFloat(Integer) (Variables|Default|GetTemperature)))
  ;[1 1 1] Set Spectral Classifcation (e.g. O5)
  (Variables|Default|SetSpectral%20Classification (Utilities|String|Append "M" (Utilities|String|ToString(Integer) (|(Abs((1-x))) (- (/ (Variables|Default|GetTemperature) 370) 1)))))
  (return Seed))

(fn SetHabitableZone
  (bind _luminosity (Variables|Default|GetLuminosity))
  (bind _temperature (Variables|Default|GetTemperature))
  (bind _returnvalue (Math|Conversions|ToFloat(Integer) _temperature))
  (bind _returnvalue_2 (Math|Float|Clamp(Float) _luminosity 2.0 25.0))
  (bind _returnvalue_3 (* _returnvalue_2 _returnvalue))
  (Variables|Default|SetMin%20Habitable%20Zone _returnvalue_3)
  (Variables|Default|SetMax%20Habitable%20Zone (+ _returnvalue_3 (/ _returnvalue_3 5.0))))